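; BP_CameraPawn is a camera pawn with a zoom level that drives both distance and tilt.
; SetCameraZoomLevel takes a normalized value and lerps the spring arm length from max to min distance, storing it as FocusDistance.
; The same value lerps the arm's pitch between its min and max, so the viewing angle changes with zoom.
; The construction script only clamps FocusDistance to the distance limits.
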(fn ConstructionScript
  (Variables|Camera|SetFocusDistance (Math|Float|Clamp(Float) (Variables|Camera|GetFocusDistance) (Variables|Camera|GetMinDistance) (Variables|Camera|GetMaxDistance))))

(fn SetCameraZoomLevel
  (params (Distance :type Float%20%28single-precision%29))
  (bind _springarm1 (Variables|Camera|GetSpringArm1))
  (bind _maxdistance (Variables|Camera|GetMaxDistance))
  (bind _mindistance (Variables|Camera|GetMinDistance))
  (bind _returnvalue (Math|Float|Lerp _maxdistance _mindistance Distance))
  (LocalVariables|SetNormalzedFocusDistance Distance)
  ;[1 1 1] Camera Distance
  (Variables|Camera|SetFocusDistance _returnvalue)
  (Variables|/Script/Engine.SpringArmComponent|SetTargetArmLength _springarm1 _returnvalue)
  ;[1 1 1] Camera Rotation
  (Transformation|SetRelativeRotation _springarm1 (Class|KismetMathLibrary|MakeRot (Math|Float|Lerp (Variables|Camera|GetMinPitch) (Variables|Camera|GetMaxPitch) Distance) (Variables|Camera|GetYaw) (Variables|Camera|GetRoll)) false))