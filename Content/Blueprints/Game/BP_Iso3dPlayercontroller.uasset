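; BP_Iso3dPlayercontroller is a player controller that pans, rotates and zooms an isometric-style camera pawn.
; Input events accumulate yaw and clamped zoom, which the CamZoom axis event pushes to BP_CameraPawn.
; Tick feeds yaw-rotated movement input to the pawn from movement axes or, while dragging, from eased normalized mouse position scaled by drag speed.
; Drag press and release also swap the hand cursor.
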(event `InputAction|CamZoomIn`
  ;[1 1 1] Zoom Level
  ;;[1 1 1] Set Zoom In
  (:`Pressed`
    (set `self.CameraZoom` (`KismetMathLibrary.FClamp` (+ (`self.CameraZoom`) 0.1)))))

(event `InputAction|CamZoomOut`
  ;[1 1 1] Zoom Level
  ;;[1 1 1] Set Zoom Out
  (:`Pressed`
    (set `self.CameraZoom` (`KismetMathLibrary.FClamp` (+ (`self.CameraZoom`) -0.1)))))

(event `InputAxis|CamZoom`
  (params (AxisValue :type "Float (single-precision)"))
  ;[1 1 1] Zoom Level
  (set `self.CameraZoom` (`KismetMathLibrary.FClamp` (+ AxisValue (`self.CameraZoom`))))
  (bind _asbp_camerapawn_c (cast `/Game/Blueprints/Game/BP_CameraPawn` (`self.GetControlledPawn`)))
  (set `/Game/Blueprints/Game/BP_CameraPawn.Yaw` (`self.CameraYaw`) _asbp_camerapawn_c)
  (`/Game/Blueprints/Game/BP_CameraPawn.SetCameraZoomLevel` _asbp_camerapawn_c (`self.CameraZoom`)))

(event `InputAxis|CamRotate`
  (params (AxisValue :type "Float (single-precision)"))
  ;[1 1 1] Gets Camera Rotation
  (set `self.CameraYaw` (+ AxisValue (`self.CameraYaw`))))

(event `InputAction|CamDragView` :consume false
  ;[1 1 1] Detect User draging
  (:`Pressed`
    (set `self.MouseDrag` true)
    (set `self.CurrentMouseCursor` "GrabHand"))
  (:`Released`
    (set `self.MouseDrag` false)
    (set `self.CurrentMouseCursor` "Hand")))

(event `self.ReceiveTick`
  (params (DeltaSeconds :type "Float (single-precision)"))
  (bind (_x _y) (`self.GetNormalizedMouse`))
  ;[1 1 1] Move the Camera
  (if (`self.MouseDrag`)
    (`Pawn.AddMovementInput` (`self.GetControlledPawn`) (`KismetMathLibrary.RotateAngleAxis` (`KismetMathLibrary.MakeVector` (`KismetMathLibrary.FInterpEaseInOut` 1.0 -1.0 _y 2.0) (`KismetMathLibrary.FInterpEaseInOut` -1.0 1.0 _x 2.0)) (`self.CameraYaw`) (0.0 0.0 1.0)) (`self.CameraDragSpeed`))
    (else
      (`Pawn.AddMovementInput` (`self.GetControlledPawn`) (`KismetMathLibrary.RotateAngleAxis` (`KismetMathLibrary.MakeVector` (`self.GetInputAxisValue`) (`self.GetInputAxisValue`)) (`self.CameraYaw`) (0.0 0.0 1.0)) 1.0))))

(fn `UserConstructionScript`
  (set `self.MouseDrag` false))