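; Player controller for a strategy-style camera, handling zoom, panning and rotation of the controlled pawn.
; Zoom keys and mouse wheel step a clamped value that the CamZoom axis event maps to spring arm length and pitch.
; Panning combines movement axes with screen-edge mouse scrolling, rotated by camera yaw so it follows the view.
; The rotate axis accumulates that yaw and applies it to the pawn's root.
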(event `InputAction|CamZoomOut`
  ;[1 1 1] Set Zoom Level
  ;;[1 1 1] Set Zoom Out
  (:`Pressed`
    (set `self.CameraZoom` (`KismetMathLibrary.FClamp` (+ (`self.CameraZoom`) 0.1)) :!label _label)))

(event `InputAction|CamZoomIn`
  ;[1 1 1] Set Zoom Level
  ;;[1 1 1] Set Zoom In
  (:`Pressed`
    (set `self.CameraZoom` (`KismetMathLibrary.FClamp` (+ (`self.CameraZoom`) -0.1)) :!label _label_2)))

(event `Key|MouseScrollDown`
  ;[1 1 1] Set Zoom Level
  ;;[1 1 1] Set Zoom Out
  (:`Pressed`
    (goto _label)))

(event `Key|MouseScrollUp`
  ;[1 1 1] Set Zoom Level
  ;;[1 1 1] Set Zoom In
  (:`Pressed`
    (goto _label_2)))

(event `InputAxis|CamZoom`
  (params (AxisValue :type "Float (single-precision)"))
  (bind _mincameradistance (`self.MinCameraDistance`))
  (bind _camerazoom (`self.CameraZoom`))
  ;[1 1 1] Set Zoom Level
  (set `self.CameraZoom` (+ (`self.CameraZoom`) 0.0))
  (for _array_element (`SceneComponent.GetChildrenComponents` (`self.K2_GetRootComponent` (`self.GetControlledPawn`)) true)
    (bind _asspringarmcomponent (cast `SpringArmComponent` _array_element))
    (set `SpringArmComponent.TargetArmLength` (+ (* _camerazoom (- (`self.MaxCameraDistance`) _mincameradistance)) _mincameradistance) _asspringarmcomponent)
    (`SceneComponent.SetRelativeRotation` _asspringarmcomponent (`KismetMathLibrary.MakeRot` (+ (* _camerazoom -30.0) -30.0)) false)))

(event `InputAxis|CamMoveLateral`
  (params (AxisValue :type "Float (single-precision)"))
  (bind (_locationx _locationy) (`self.GetMousePosition`))
  (bind (_sizex _sizey) (`self.GetViewportSize`))
  (bind _returnvalue (/ _locationx (`KismetMathLibrary.Conv_IntToDouble` _sizex)))
  (bind _returnvalue_2 (/ _locationy (`KismetMathLibrary.Conv_IntToDouble` _sizey)))
  (bind _returnvalue_3 (> _returnvalue_2 0.0))
  (bind _returnvalue_4 (> _returnvalue 0.0))
  ;[1 1 1] Move the Camera
  (`Pawn.AddMovementInput` (`self.GetControlledPawn`) (`KismetMathLibrary.RotateAngleAxis` (`KismetMathLibrary.MakeVector` (+ (`self.GetInputAxisValue`) (* (`KismetMathLibrary.Conv_BoolToDouble` (and (>= _returnvalue_2 0.95) _returnvalue_3)) -1.0) (`KismetMathLibrary.Conv_BoolToDouble` (and (<= _returnvalue_2 0.05) _returnvalue_3))) (+ (`self.GetInputAxisValue`) (`KismetMathLibrary.Conv_BoolToDouble` (and (>= _returnvalue 0.95) _returnvalue_4)) (* (`KismetMathLibrary.Conv_BoolToDouble` (and (<= _returnvalue 0.05) _returnvalue_4)) -1.0))) (`self.CameraYaw`) (0.0 0.0 1.0)) 1.0 :!label _label_3))

(event `InputAxis|CamMoveFrontBack`
  (params (AxisValue :type "Float (single-precision)"))
  ;[1 1 1] Move the Camera
  (goto _label_3))

(event `InputAxis|CamRotate`
  (params (AxisValue :type "Float (single-precision)"))
  (bind _returnvalue (+ AxisValue (`self.CameraYaw`)))
  (set `self.CameraYaw` _returnvalue)
  (`SceneComponent.SetRelativeRotation` (`self.K2_GetRootComponent` (`self.GetControlledPawn`)) (`KismetMathLibrary.MakeRot` 0.0 _returnvalue) false))

(fn `UserConstructionScript`)